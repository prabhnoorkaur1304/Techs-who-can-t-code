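; Blueprint for the blue sprite character, which handles talking through a Talk event.
; Each Talk increments TalkIndex and prints that entry of the Dialogue array to the screen.
; It then creates a UI widget for the first player controller and adds it to the viewport if none exists yet.
; The branch condition is fixed to true, leaving the dialogue length check disconnected, so the index is unbounded.
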(event `/Game/Character/Sprites/BlueCharacter/BPI_BlueCharacter_Dialogue.Talk`
  (`/Engine/EditorBlueprintResources/StandardMacros.IncrementInt` (`self.TalkIndex`)
    (:`  `
      (if true
        (`KismetSystemLibrary.PrintString` (`|GetArrayItem` (`self.Dialogue`) (`self.TalkIndex`)))
        (`self.UI`
          (:`then`)
          (:`else`
            (bind _returnvalue (`|CreateWidget` null (`GameplayStatics.GetPlayerController` 0)))
            (bind _output_get (set `self.UI` _returnvalue))
            (`UserWidget.AddToViewport` _output_get 0)))))))

(fn `UserConstructionScript`)